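; BP_Character is a Character Blueprint that provides basic movement, look, jump and death behavior.
; Movement events add input along control-yaw forward and right vectors, while look events divide axis values by sensitivity variables before adding yaw and pitch.
; JumpPress calls Jump and Death destroys the actor.
; CharacterRef returns the character itself, while ControllerRef returns no value.
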(event Custom|Death
  (Actor|DestroyActor))

(event EventMoveForward
  (params (Axis%20Value :type Float%20%28single-precision%29))
  ;[1 1 1] Movement
  (Pawn|Input|AddMovementInput (Math|Vector|GetForwardVector (Math|Rotator|MakeRotator 0.0 0.0 (.yaw (Pawn|GetControlRotation :!class /Script/Engine.Pawn)))) Axis%20Value false))

(event EventMoveRight
  (params (Axis%20Value :type Float%20%28single-precision%29))
  ;[1 1 1] Movement
  (Pawn|Input|AddMovementInput (Math|Vector|GetRightVector (Math|Rotator|MakeRotator 0.0 0.0 (.yaw (Pawn|GetControlRotation :!class /Script/Engine.Pawn)))) Axis%20Value false))

(event EventLookRight
  (params (Axis%20Value :type Float%20%28single-precision%29))
  ;[1 1 1] Movement
  (Pawn|Input|AddControllerYawInput (/ Axis%20Value (Variables|Default|GetLeftRightSensitvity))))

(event EventLookUp
  (params (Axis%20Value :type Float%20%28single-precision%29))
  ;[1 1 1] Movement
  (Pawn|Input|AddControllerPitchInput (/ Axis%20Value (Variables|Default|GetUpDownSensitivity))))

(event EventJumpPress
  ;[1 1 1] Movement
  (Character|Jump))

(fn ConstructionScript)

(fn CharacterRef
  (return self))

(fn ControllerRef
  (return 0))