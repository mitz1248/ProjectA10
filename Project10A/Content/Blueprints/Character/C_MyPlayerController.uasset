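; Player controller for a 1v1 mode that spawns, initializes and possesses its character, forwarding stick and jump input to the pawn through message calls.
; Timer events disable character movement while showing a countdown widget, then restore walking and remove it.
; AnyDamage sets Health to damage minus Health, notifying the game mode and killing the character at zero or below.
; The G key applies self-damage.
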(event Custom|Timer
  ;[1 1 1] GameMode
  (bind _character (Class|ICharacter|CharacterRef(Message) (Pawn|GetControlledPawn)))
  (CallFunction|TurnMovementOff (Variables|/Script/Engine.Character|GetCharacterMovement _character)))

(event Custom|FinishedTimer
  ;[1 1 1] GameMode
  (bind _character (Class|ICharacter|CharacterRef(Message) (Pawn|GetControlledPawn)))
  (CallFunction|TurnMovementon (Variables|/Script/Engine.Character|GetCharacterMovement _character)))

(event Game|Damage|EventAnyDamage
  (params (Damage :type Float%20%28single-precision%29) (DamageType :type Damage%20Type%20Object%20Reference) (InstigatedBy :type Controller%20Object%20Reference) (DamageCauser :type Actor%20Object%20Reference))
  (bind _output_get (Variables|Default|SetHealth (- Damage (Variables|Default|GetHealth))))
  (if (<= _output_get 0.0)
    (bind _1v1ref (Class|IGameMode1v1|1v1Ref(Message) (Game|GetGameMode)))
    (Class|IGameMode1v1|Death(Message) _1v1ref self)
    (bind _character (Class|ICharacter|CharacterRef(Message) (Pawn|GetControlledPawn)))
    (Default|Death _character)))

(event EventInit
  (params (spawnTransform :type Transform))
  ;[1 1 1] InitChain
  (bind _returnvalue (Game|SpawnActorfromClass (Variables|Default|GetClass) spawnTransform "Undefined" 0 0))
  (Class|IGameMode1v1|Init(Message) _returnvalue)
  (Pawn|Possess _returnvalue))

(event Input|ActionEvents|InputActionJump
  (params (Key :type Key%20Structure))
  (bind _returnvalue (Pawn|GetControlledPawn))
  ;[1 1 1] Input
  (:Pressed
    (Class|IController|JumpPress(Message) _returnvalue))
  (:Released
    (Class|IController|JumpRelease(Message) _returnvalue)))

(event Input|AxisEvents|InputAxisLeftStickX
  (params (AxisValue :type Float%20%28single-precision%29))
  ;[1 1 1] Input
  (Class|IController|MoveRight(Message) (Pawn|GetControlledPawn) AxisValue))

(event Input|AxisEvents|InputAxisLeftStickY
  (params (AxisValue :type Float%20%28single-precision%29))
  ;[1 1 1] Input
  (Class|IController|MoveForward(Message) (Pawn|GetControlledPawn) AxisValue))

(event Input|AxisEvents|InputAxisRightStickX
  (params (AxisValue :type Float%20%28single-precision%29))
  ;[1 1 1] Input
  (Class|IController|LookRight(Message) (Pawn|GetControlledPawn) AxisValue))

(event Input|AxisEvents|InputAxisRightStickY
  (params (AxisValue :type Float%20%28single-precision%29))
  ;[1 1 1] Input
  (Class|IController|LookUp(Message) (Pawn|GetControlledPawn) AxisValue))

(event Input|KeyboardEvents|G
  (params (Key :type Key%20Structure))
  (:Pressed
    (Game|Damage|ApplyDamage self 1e+02 0 0)))

(fn ConstructionScript)

(fn TurnMovementOff
  (params (CharacterMove :type Character%20Movement%20Component%20Object%20Reference))
  (Pawn|Components|CharacterMovement|SetMovementMode CharacterMove "MOVE_None" 0)
  (bind _returnvalue (UserInterface|CreateWidget "/Game/Blueprints/UI/Timer.Timer_C" self))
  (bind _output_get (Variables|Default|SetTimerHUDRef _returnvalue))
  (UserInterface|Viewport|AddtoPlayerScreen _output_get))

(fn TurnMovementon
  (params (Character%20Move :type Character%20Movement%20Component%20Object%20Reference))
  (Pawn|Components|CharacterMovement|SetMovementMode Character%20Move "MOVE_Walking" 0)
  (Widget|RemovefromParent (Variables|Default|GetTimerHUDRef)))

(fn 1v1Ref
  (return 0))

(fn ControllerRef
  (return self))