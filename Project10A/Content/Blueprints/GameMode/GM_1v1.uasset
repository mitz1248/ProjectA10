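; GM_1v1 is a match-state Game Mode for 1v1 play, still largely stubbed.
; New players are restarted and added to a Controllers array, with spawns always resolving to the first CustomPlayerStart found.
; The match is always ready to start and ready to end whenever exactly one controller is stored.
; Logout and match-state handlers are empty, and nothing removes controllers from the array.
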(event EventBeginPlay)

(event EventHandleStartingNewPlayer
  (params (NewPlayer :type Player%20Controller%20Object%20Reference))
  ;[1 1 1] SpawnsPlayerAndAddsToArray
  (Class|GameModeBase|RestartPlayer NewPlayer)
  (Utilities|Array|AddUnique (Variables|Default|GetControllers) NewPlayer))

(event EventPostLogin
  (params (NewPlayer :type Player%20Controller%20Object%20Reference)))

(event EventOnLogout
  (params (ExitingController :type Controller%20Object%20Reference)))

(event EventOnSetMatchState
  (params (NewState :type Name :default "None"))
  (switch name NewState))

(fn ConstructionScript)

(fn FindPlayerStart
  (params (Player :type Controller%20Object%20Reference) (IncomingName :type String))
  (bind _outactors (Actor|GetAllActorsOfClass "/Game/Blueprints/GameMode/CustomPlayerStart.CustomPlayerStart_C"))
  (return (Utilities|Array|Get(acopy) _outactors)))

(fn ReadytoStartMatch
  (for _array_element (Variables|Default|GetControllers)
    _)
  (return true))

(fn ReadytoEndMatch
  (return (== (Utilities|Array|Length (Variables|Default|GetControllers)) 1)))

(fn ControllerRef
  (return 0))